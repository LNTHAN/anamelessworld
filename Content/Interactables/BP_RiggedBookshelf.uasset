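; BP_RiggedBookshelf is an interactable bookshelf that topples over when detonated.
; OnDetonated stores the actor's rotation, then the Topple timeline lerps the Pivot component's relative rotation from that value toward a 90-degree pitch combined with it.
; When the timeline finishes, it triggers a camera shake on player 0's pawn if that pawn is a TacticalCameraPawn.
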(event EventOnDetonated
  (Variables|Default|SetInitialRotation (Transformation|GetActorRotation))
  (bind _alpha (Timeline|Topple PlayFromStart)
    (:Update
      (Transformation|SetRelativeRotation (Variables|Default|GetPivot) (Math|Rotator|Lerp(Rotator) (Variables|Default|GetInitialRotation) (Math|Rotator|CombineRotators (Math|Rotator|MakeRotator 0.0 9e+01 0.0) (Variables|Default|GetInitialRotation)) _alpha) false false))
    (:Finished
      (bind _astactical_camera_pawn (Utilities|Casting|CastToTacticalCameraPawn (Pawn|GetControlledPawn (Game|GetPlayerController 0))))
      (Class|TacticalCameraPawn|TriggerShake _astactical_camera_pawn))))

(fn ConstructionScript)